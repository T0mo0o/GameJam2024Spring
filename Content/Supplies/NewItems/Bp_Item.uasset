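; Base pickup actor for a world item that the player can interact with to add to the inventory.
; On BeginPlay it fills an unset ItemObject from GetDefaultItemObject, which returns nothing here.
; Interact passes ItemObject to TryAddItem on the InventoryComponent of player 0's BP_ThirdPersonCharacter.
; The actor destroys itself on success and prints a red debug string on failure.
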(event EventBeginPlay
  (if (not (Utilities|IsValid (Variables|Private|GetItemObject)))
    (bind _itemobject (Private|GetDefaultItemObject))
    (Variables|Private|SetItemObject _itemobject)))

(event EventInteract
  (bind _asbp_third_person_character (Utilities|Casting|CastToBP_ThirdPersonCharacter (Game|GetPlayerCharacter 0)))
  (bind _added (Default|TryAddItem (Variables|/Game/ThirdPerson/Blueprints/BP_ThirdPersonCharacter.BP_ThirdPersonCharacter_C|GetInventory_Component _asbp_third_person_character) (Variables|Private|GetItemObject)))
  (if _added
    (Actor|DestroyActor)
    (else
      (Development|PrintString "Hello" true true "(R=1.000000,G=0.000000,B=0.019891,A=1.000000)"))))

(fn ConstructionScript)

(fn GetDefaultItemObject
  (return 0))