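; BP_Item_Object represents an item in the inventory system, holding its dimensions, icons, item class and rotation state.
; Rotate toggles the Rotated flag, which IsRotated exposes.
; GetDimensions swaps X and Y while rotated, and GetIcon returns a separate pre-rotated icon, so callers receive values that match the current orientation.
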(fn GetDimensions
  (bind _dimensions (Variables|Private|GetDimensions))
  (if (Variables|Default|GetRotated)
    (return (Utilities|Struct|MakeIntPoint (.y _dimensions) (.x _dimensions)))
    (else
      (return (Variables|Private|GetDimensions)))))

(fn GetIcon
  (return (select (Variables|Default|GetRotated) (Variables|Private|GetIconRotated) (Variables|Private|GetIcon))))

(fn GetItemClass
  (return (Variables|Private|GetItemClass)))

(fn Rotate
  (Variables|Default|SetRotated (not (Variables|Default|GetRotated))))

(fn IsRotated
  (return (Variables|Default|GetRotated)))